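; BP_BrawlGameMode is the game mode for a two-player brawl, spawning each player's selected character and running an opening countdown.
; BeginPlay shows the HUD and countdown widgets, starts the one-second countdown timer and points the first controller at BP_Camera.
; PostLogin records controllers, then after a delay uses their index to choose input mapping, saved character class and PlayerStart before possession.
; A local CreatePlayer loop is present but disconnected.
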(event Custom|Take%20Countdown
  (Math|Integer|DecrementInt (Variables|Default|GetCount)
    (:%20%20
      (Rendering|Components|TextRender|SetText (Variables|/Game/UI_Widgets/WBP_Countdown.WBP_Countdown_C|GetCountDownText (Variables|Default|GetCountDownWidget)) (Utilities|Text|ToText(Integer) (Variables|Default|GetCount)))
      (if (<= (Variables|Default|GetCount) 0)
        (Utilities|Time|ClearandInvalidateTimerbyHandle (Variables|Default|GetTimerClean))
        (Widget|RemovefromParent (Variables|Default|GetCountDownWidget))))))

(event Custom|ActuallyStartPlayer
  (params (PlayerController :type Player%20Controller%20Object%20Reference))
  (bind _controllers (Variables|Default|GetControllers))
  (bind _returnvalue (Utilities|Array|FindItem _controllers PlayerController))
  (Input|AddMappingContext (PlayerController|LocalPlayerSubsystems|GetEnhancedInputLocalPlayerSubsystem PlayerController) (Utilities|Select :Index _returnvalue :Option%200 "/Game/CoreGame/Input/IMC_Player1.IMC_Player1" :Option%201 "/Game/CoreGame/Input/IMC_Player2.IMC_Player2") 0 (Utilities|Struct|MakeModifyContextOptions true false))
  (bind _returnvalue_2 (Utilities|GetPlayerCharacterClass _returnvalue))
  (bind _returnvalue_3 (Game|SpawnActorfromClass _returnvalue_2 (Transformation|GetActorTransform (Class|GameModeBase|FindPlayerStart PlayerController (Utilities|String|ToString(Integer) _returnvalue))) "AdjustIfPossibleButAlwaysSpawn" "MultiplyWithRoot" PlayerController 0))
  (Pawn|Possess PlayerController _returnvalue_3))

(event EventPostLogin
  (params (NewPlayer :type Player%20Controller%20Object%20Reference))
  (Utilities|Array|AddUnique (Variables|Default|GetControllers) NewPlayer)
  (Utilities|FlowControl|Delay 2.0)
  (CallFunction|ActuallyStartPlayer NewPlayer))

(event EventBeginPlay
  (bind _ascore_game_instance (Utilities|Casting|CastToCoreGameInstance (Game|GetGameInstance)))
  (Variables|Default|SetGameInstanceRef _ascore_game_instance)
  (bind _returnvalue (UserInterface|CreateWidget "/Game/UI_Widgets/WBP_Countdown.WBP_Countdown_C"))
  (bind _output_get (Variables|Default|SetCountDownWidget _returnvalue))
  (bind _returnvalue_2 (Utilities|Time|SetTimerbyEvent (delegate Custom|Take%20Countdown) 1.0 true))
  (Variables|Default|SetTimerClean _returnvalue_2)
  (bind _returnvalue_3 (UserInterface|CreateWidget "/Game/UI_Widgets/WBP_HudUI.WBP_HudUI_C"))
  (UserInterface|Viewport|AddtoViewport _returnvalue_3 0)
  (bind _returnvalue_4 (Actor|GetActorOfClass "/Game/Characters/BP_Actors/BP_Camera.BP_Camera_C"))
  (Game|Player|SetViewTargetwithBlend (Utilities|Array|Get(acopy) (Variables|Default|GetControllers)) _returnvalue_4 0.0 "VTBlend_Linear" 0.0 false))

(fn ConstructionScript)

(fn FindPlayerStart
  (params (Player :type Controller%20Object%20Reference) (IncomingName :type String))
  (if (.bSuccess (Utilities|Casting|CastToPlayerController Player))
    (if (== (Utilities|Array|Length (Variables|Default|GetPlayerStarts)) 0)
      (bind _outactors (Actor|GetAllActorsOfClass "/Script/Engine.PlayerStart"))
      (bind _output_get (Variables|Default|SetPlayerStarts _outactors)))
    (return (Utilities|Array|Get(acopy) _output_get (Math|Conversions|ToInteger(Byte) IncomingName)))
    (else
      (return 0))))