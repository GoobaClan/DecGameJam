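; Monk player character that adds a parry and a haymaker as unique attacks and spawns a monk hat attached to its head socket.
; Enhanced Input events call these moves and the shared punch, kick, block, jump and emote functions.
; Both unique attacks play a one-off mesh animation, then restore the Animation Blueprint after timed delays, with parry also holding a Parrying flag.
; Incoming damage is forwarded to TakeAnyDamage.
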(event Custom|Haymaker
  (Components|Animation|PlayAnimation (Variables|Character|GetMesh) "/Game/Characters/The_CharacterAnims/Monk/Flyingpunch.Flyingpunch" false)
  (Utilities|FlowControl|Delay 0.8)
  (Utilities|FlowControl|Delay 1.2)
  (Components|Animation|SetAnimationMode (Variables|Character|GetMesh) "AnimationBlueprint"))

(event Custom|OnTakeAnyDamage_Event
  (params (DamagedActor :type Actor%20Object%20Reference) (Damage :type Float%20%28single-precision%29) (DamageType :type Damage%20Type%20Object%20Reference) (InstigatedBy :type Controller%20Object%20Reference) (DamageCauser :type Actor%20Object%20Reference))
  (CallFunction|TakeAnyDamage Damage))

(event Custom|Parry
  (Variables|Default|Setparrying true)
  (Components|Animation|PlayAnimation (Variables|Character|GetMesh) "/Game/Characters/The_CharacterAnims/Monk/ParryAnimation.ParryAnimation" false)
  (Utilities|FlowControl|Delay 1.4)
  (Variables|Default|Setparrying false)
  (Components|Animation|SetAnimationMode (Variables|Character|GetMesh) "AnimationBlueprint"))

(event Input|EnhancedActionEvents|EnhancedInputActionIA_Jump
  (params (ActionValue :type Boolean) (ElapsedSeconds :type Float%20%28double-precision%29) (TriggeredSeconds :type Float%20%28double-precision%29) (InputAction :type Input%20Action%20Object%20Reference :default "/Game/CoreGame/Input/Actions/IA_Jump.IA_Jump"))
  (:Triggered
    (CallFunction|DoJump))
  (:Completed
    (CallFunction|StopJump)))

(event Input|EnhancedActionEvents|EnhancedInputActionIA_UniqueAttack2
  (params (ActionValue :type Boolean) (ElapsedSeconds :type Float%20%28double-precision%29) (TriggeredSeconds :type Float%20%28double-precision%29) (InputAction :type Input%20Action%20Object%20Reference :default "/Game/CoreGame/Input/Actions/IA_UniqueAttack2.IA_UniqueAttack2"))
  (:Triggered
    (CallFunction|Haymaker)))

(event Input|EnhancedActionEvents|EnhancedInputActionIA_Kick
  (params (ActionValue :type Boolean) (ElapsedSeconds :type Float%20%28double-precision%29) (TriggeredSeconds :type Float%20%28double-precision%29) (InputAction :type Input%20Action%20Object%20Reference :default "/Game/CoreGame/Input/Actions/IA_Kick.IA_Kick"))
  (:Triggered
    (CallFunction|DoKick)))

(event Input|EnhancedActionEvents|EnhancedInputActionIA_Punch
  (params (ActionValue :type Boolean) (ElapsedSeconds :type Float%20%28double-precision%29) (TriggeredSeconds :type Float%20%28double-precision%29) (InputAction :type Input%20Action%20Object%20Reference :default "/Game/CoreGame/Input/Actions/IA_Punch.IA_Punch"))
  (:Triggered
    (CallFunction|DoPunch)))

(event Input|EnhancedActionEvents|EnhancedInputActionIA_UniqueAttack1
  (params (ActionValue :type Boolean) (ElapsedSeconds :type Float%20%28double-precision%29) (TriggeredSeconds :type Float%20%28double-precision%29) (InputAction :type Input%20Action%20Object%20Reference :default "/Game/CoreGame/Input/Actions/IA_UniqueAttack1.IA_UniqueAttack1"))
  (:Triggered
    (CallFunction|Parry)))

(event Input|EnhancedActionEvents|EnhancedInputActionIA_Emote
  (params (ActionValue :type Boolean) (ElapsedSeconds :type Float%20%28double-precision%29) (TriggeredSeconds :type Float%20%28double-precision%29) (InputAction :type Input%20Action%20Object%20Reference :default "/Game/CoreGame/Input/Actions/IA_Emote.IA_Emote"))
  (:Triggered
    (CallFunction|DoEmote)))

(event Input|EnhancedActionEvents|EnhancedInputActionIA_Pause
  (params (ActionValue :type Boolean) (ElapsedSeconds :type Float%20%28double-precision%29) (TriggeredSeconds :type Float%20%28double-precision%29) (InputAction :type Input%20Action%20Object%20Reference :default "/Game/CoreGame/Input/Actions/IA_Pause.IA_Pause")))

(event Input|EnhancedActionEvents|EnhancedInputActionIA_Block
  (params (ActionValue :type Boolean) (ElapsedSeconds :type Float%20%28double-precision%29) (TriggeredSeconds :type Float%20%28double-precision%29) (InputAction :type Input%20Action%20Object%20Reference :default "/Game/CoreGame/Input/Actions/IA_Block.IA_Block"))
  (:Triggered
    (CallFunction|DoBlock))
  (:Canceled
    (CallFunction|DoBlockStop :!label _label))
  (:Completed
    (goto _label)))

(event EventBeginPlay
  (Utilities|FlowControl|DelayUntilNextTick)
  (bind _returnvalue (Game|SpawnActorfromClass "/Game/Characters/Hats/BP_Monkhat.BP_Monkhat_C" (Transformation|GetSocketTransform (Variables|Character|GetMesh) "HeadSocket" "RTS_World") "Undefined" "MultiplyWithRoot" 0 0))
  (Transformation|AttachComponentToComponent _returnvalue (Variables|Character|GetMesh) "HeadSocket" "SnapToTarget" "SnapToTarget" "SnapToTarget" true))

(fn ConstructionScript
  (|CallParentFunction))