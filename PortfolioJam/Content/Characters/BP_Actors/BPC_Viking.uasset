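; BPC_Viking is a playable Viking character with a greataxe, two unique attacks and shared combat moves.
; It spawns and attaches the axe to a mesh socket one tick after BeginPlay, and forwards damage and standard Enhanced Input actions to functions defined elsewhere.
; Headbutt plays an animation and runs a debug-drawn box trace whose result is unused.
; Charge temporarily boosts walk speed with attached smoke until a timer calls StopCharge.
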(event Custom|Charge
  (Variables|Default|SetisCharging true)
  (Variables|/Script/Engine.CharacterMovementComponent|SetMaxWalkSpeed (Variables|Character|GetCharacterMovement) 1.2e+03)
  (Effects|SpawnEmitterAttached "/Game/StarterContent/Particles/P_Smoke.P_Smoke" (Variables|Default|GetCapsuleComponent) "None")
  (Utilities|Time|SetTimerbyFunctionName 0 "StopCharge" 3.0))

(event Custom|OnTakeAnyDamage_Event
  (params (DamagedActor :type Actor%20Object%20Reference) (Damage :type Float%20%28single-precision%29) (DamageType :type Damage%20Type%20Object%20Reference) (InstigatedBy :type Controller%20Object%20Reference) (DamageCauser :type Actor%20Object%20Reference))
  (CallFunction|TakeAnyDamage Damage))

(event Custom|Headbutt
  (Components|Animation|PlayAnimation (Variables|Character|GetMesh) 0 false)
  (Collision|BoxTraceByChannel (Transformation|GetSocketLocation (Variables|Default|GetStartAttack) "None") (Transformation|GetSocketLocation (Variables|Default|GetEndAttack) "None") "0.000000,50.000000,50.000000" (Variables|/Script/Engine.SceneComponent|GetRelativeRotation (Variables|Default|GetCapsuleComponent)) "TraceTypeQuery1" false 0 "Persistent"))

(event Input|EnhancedActionEvents|EnhancedInputActionIA_UniqueAttack1
  (params (ActionValue :type Boolean) (ElapsedSeconds :type Float%20%28double-precision%29) (TriggeredSeconds :type Float%20%28double-precision%29) (InputAction :type Input%20Action%20Object%20Reference :default "/Game/CoreGame/Input/Actions/IA_UniqueAttack1.IA_UniqueAttack1"))
  (:Triggered
    (CallFunction|Headbutt)))

(event Input|EnhancedActionEvents|EnhancedInputActionIA_UniqueAttack2
  (params (ActionValue :type Boolean) (ElapsedSeconds :type Float%20%28double-precision%29) (TriggeredSeconds :type Float%20%28double-precision%29) (InputAction :type Input%20Action%20Object%20Reference :default "/Game/CoreGame/Input/Actions/IA_UniqueAttack2.IA_UniqueAttack2"))
  (:Triggered
    (CallFunction|Charge)))

(event Input|EnhancedActionEvents|EnhancedInputActionIA_Kick
  (params (ActionValue :type Boolean) (ElapsedSeconds :type Float%20%28double-precision%29) (TriggeredSeconds :type Float%20%28double-precision%29) (InputAction :type Input%20Action%20Object%20Reference :default "/Game/CoreGame/Input/Actions/IA_Kick.IA_Kick"))
  (:Triggered
    (CallFunction|DoKick)))

(event Input|EnhancedActionEvents|EnhancedInputActionIA_Punch
  (params (ActionValue :type Boolean) (ElapsedSeconds :type Float%20%28double-precision%29) (TriggeredSeconds :type Float%20%28double-precision%29) (InputAction :type Input%20Action%20Object%20Reference :default "/Game/CoreGame/Input/Actions/IA_Punch.IA_Punch"))
  (:Triggered
    (CallFunction|DoPunch)))

(event Input|EnhancedActionEvents|EnhancedInputActionIA_Jump
  (params (ActionValue :type Boolean) (ElapsedSeconds :type Float%20%28double-precision%29) (TriggeredSeconds :type Float%20%28double-precision%29) (InputAction :type Input%20Action%20Object%20Reference :default "/Game/CoreGame/Input/Actions/IA_Jump.IA_Jump"))
  (:Triggered
    (CallFunction|DoJump))
  (:Completed
    (CallFunction|StopJump)))

(event Input|EnhancedActionEvents|EnhancedInputActionIA_Emote
  (params (ActionValue :type Boolean) (ElapsedSeconds :type Float%20%28double-precision%29) (TriggeredSeconds :type Float%20%28double-precision%29) (InputAction :type Input%20Action%20Object%20Reference :default "/Game/CoreGame/Input/Actions/IA_Emote.IA_Emote"))
  (:Triggered
    (CallFunction|DoEmote)))

(event Input|EnhancedActionEvents|EnhancedInputActionIA_Pause
  (params (ActionValue :type Boolean) (ElapsedSeconds :type Float%20%28double-precision%29) (TriggeredSeconds :type Float%20%28double-precision%29) (InputAction :type Input%20Action%20Object%20Reference :default "/Game/CoreGame/Input/Actions/IA_Pause.IA_Pause")))

(event Input|EnhancedActionEvents|EnhancedInputActionIA_Block
  (params (ActionValue :type Boolean) (ElapsedSeconds :type Float%20%28double-precision%29) (TriggeredSeconds :type Float%20%28double-precision%29) (InputAction :type Input%20Action%20Object%20Reference :default "/Game/CoreGame/Input/Actions/IA_Block.IA_Block"))
  (:Triggered
    (CallFunction|DoBlock))
  (:Canceled
    (CallFunction|DoBlockStop :!label _label))
  (:Completed
    (goto _label)))

(event EventBeginPlay
  (Utilities|FlowControl|DelayUntilNextTick)
  (bind _returnvalue (Game|SpawnActorfromClass "/Game/Characters/The_Character_Meshs/Viking/BP_Greataxe.BP_Greataxe_C" (Transformation|GetSocketTransform (Variables|Character|GetMesh) "Axe" "RTS_World") "Undefined" "MultiplyWithRoot" 0 0))
  (Transformation|AttachComponentToComponent _returnvalue (Variables|Character|GetMesh) "Axe" "SnapToTarget" "SnapToTarget" "SnapToTarget" true))

(fn ConstructionScript
  (|CallParentFunction))

(fn StopCharge
  (Variables|Default|SetisCharging false)
  (Variables|/Script/Engine.CharacterMovementComponent|SetMaxWalkSpeed (Variables|Character|GetCharacterMovement) 6e+02))