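; Paladin character Blueprint with two greatsword attacks, Divine Smite and an arc attack, bound to Enhanced Input.
; BeginPlay spawns BP_Greatsword, attaches it to the SwordHolder socket and adds the Player 1 mapping context.
; Each attack plays an animation directly on the mesh and uses fixed Delays to time the sword's start and end calls, then returns to idle.
; Divine Smite also triggers the sword's PlayBoom mid-attack.
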(event Custom|Arc%20Attack
  (Components|Animation|PlayAnimation (Variables|Character|GetMesh) "/Game/Characters/The_CharacterAnims/Paladin/Arc.Arc" false)
  (Default|Attacking (stale EventBeginPlay _returnvalue))
  (Utilities|FlowControl|Delay 1.6)
  (Default|EndAttack (stale EventBeginPlay _returnvalue))
  (Components|Animation|PlayAnimation (Variables|Character|GetMesh) "/Game/Characters/The_CharacterAnims/Paladin/Paladin_Idle.Paladin_Idle" false))

(event Custom|Divine%20Smite
  (Components|Animation|PlayAnimation (Variables|Character|GetMesh) "/Game/Characters/The_CharacterAnims/Paladin/SmiteNew.SmiteNew" false)
  (Default|AttackingSmite (stale EventBeginPlay _returnvalue))
  (Utilities|FlowControl|Delay 3.0)
  (Default|PlayBoom (stale EventBeginPlay _returnvalue))
  (Utilities|FlowControl|Delay 1.5)
  (Default|EndAttackSmite (stale EventBeginPlay _returnvalue))
  (Components|Animation|PlayAnimation (Variables|Character|GetMesh) "/Game/Characters/The_CharacterAnims/Paladin/Paladin_Idle.Paladin_Idle" false))

(event Input|EnhancedActionEvents|EnhancedInputActionIA_UniqueAttack1
  (params (ActionValue :type Boolean) (ElapsedSeconds :type Float%20%28double-precision%29) (TriggeredSeconds :type Float%20%28double-precision%29) (InputAction :type Input%20Action%20Object%20Reference :default "/Game/CoreGame/Input/Actions/IA_UniqueAttack1.IA_UniqueAttack1"))
  (:Triggered
    (CallFunction|DivineSmite)))

(event Input|EnhancedActionEvents|EnhancedInputActionIA_UniqueAttack2
  (params (ActionValue :type Boolean) (ElapsedSeconds :type Float%20%28double-precision%29) (TriggeredSeconds :type Float%20%28double-precision%29) (InputAction :type Input%20Action%20Object%20Reference :default "/Game/CoreGame/Input/Actions/IA_UniqueAttack2.IA_UniqueAttack2"))
  (:Triggered
    (CallFunction|ArcAttack)))

(event EventBeginPlay
  (bind _returnvalue (Game|SpawnActorfromClass "/Game/Megascans/3D_Assets/Sword_uitlbiaga/BP_Greatsword.BP_Greatsword_C" (Transformation|GetSocketTransform (Variables|Character|GetMesh) "SwordHolder" "RTS_World") "Undefined" "MultiplyWithRoot" 0 0))
  (Transformation|AttachComponentToComponent _returnvalue (Variables|Character|GetMesh) "SwordHolder" "SnapToTarget" "SnapToTarget" "SnapToTarget" true)
  (Components|Animation|PlayAnimation (Variables|Character|GetMesh) "/Game/Characters/The_CharacterAnims/Paladin/Paladin_Idle.Paladin_Idle" false)
  (if true
    (bind _returnvalue_2 (CallFunction|GetInputSubSystem))
    (Utilities|IsValid _returnvalue_2
      (:Is%20Valid
        (Input|AddMappingContext _returnvalue_2 "/Game/CoreGame/Input/IMC_Player1.IMC_Player1" 0 "(bIgnoreAllPressedKeysUntilRelease=True,bForceImmediately=False)")))))

(fn ConstructionScript
  (|CallParentFunction))