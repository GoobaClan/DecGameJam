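; MR_T character Blueprint with shared fighting inputs (punch, kick, block, jump, emote) and two unique attacks, plus horns attached to its head socket on spawn.
; Bash plays a casting animation, attaches a temporary tentacle and runs a debug-drawn box trace whose result is unused.
; Pull box-traces forward after its animation and briefly shows a cable latched to any hit actor, without applying any pulling movement.
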(event Custom|Bash
  (bind _capsulecomponent (Variables|Default|GetCapsuleComponent))
  (bind _mesh (Variables|Character|GetMesh))
  (bind _returnvalue (Transformation|GetSocketTransform _mesh "Tentacle" "RTS_World"))
  (bind _relativerotation (Variables|/Script/Engine.SceneComponent|GetRelativeRotation _capsulecomponent))
  (Components|Animation|PlayAnimation (Variables|Character|GetMesh) "/Game/Characters/The_CharacterAnims/Mr_T/Magic_Spell_Casting_Anim_mixamo_com.Magic_Spell_Casting_Anim_mixamo_com" false)
  (Utilities|FlowControl|Delay 1.75)
  (Development|PrintString (Utilities|String|ToString(Float) (.yaw _relativerotation)))
  (bind _returnvalue_2 (Game|SpawnActorfromClass "/Game/Characters/The_CharacterAnims/Mr_T/BP_Tentacle.BP_Tentacle_C" (Math|Transform|MakeTransform (.location _returnvalue) (Math|Rotator|MakeRotator 0.0 0.0 (.yaw _relativerotation)) (.scale _returnvalue)) "Undefined" "MultiplyWithRoot" 0 0))
  (Transformation|AttachComponentToComponent _returnvalue_2 (Variables|Character|GetMesh) "Tentacle" "SnapToTarget" "SnapToTarget" "SnapToTarget" true)
  (Collision|BoxTraceByChannel (Transformation|GetSocketLocation (Variables|Default|GetTentacleStart) "None") (Transformation|GetSocketLocation (Variables|Default|GetTentacleEnd) "None") "0.000000,40.000000,50.000000" (Variables|/Script/Engine.SceneComponent|GetRelativeRotation (Variables|Default|GetCapsuleComponent)) "TraceTypeQuery1" false 0 "Persistent")
  (Utilities|FlowControl|Delay 1.4)
  (Actor|DestroyActor _returnvalue_2)
  (Components|Animation|SetAnimationMode (Variables|Character|GetMesh) "AnimationBlueprint"))

(event Custom|OnTakeAnyDamage_Event
  (params (DamagedActor :type Actor%20Object%20Reference) (Damage :type Float%20%28single-precision%29) (DamageType :type Damage%20Type%20Object%20Reference) (InstigatedBy :type Controller%20Object%20Reference) (DamageCauser :type Actor%20Object%20Reference))
  (CallFunction|TakeAnyDamage Damage))

(event Custom|Pull
  (bind _cable (Variables|Default|GetCable))
  (Components|Animation|PlayAnimation (Variables|Character|GetMesh) "/Game/Characters/The_CharacterAnims/Mr_T/Two_Hand_Spell_Casting_Anim_mixamo_com.Two_Hand_Spell_Casting_Anim_mixamo_com" false)
  (Utilities|FlowControl|Delay 1.5)
  (bind (_outhit _returnvalue) (Collision|BoxTraceByChannel (Transformation|GetSocketLocation (Variables|Default|GetTentacleStart) "None") (Transformation|GetSocketLocation (Variables|Default|Getlatch%20End) "None") "0.000000,200.000000,50.000000" (Variables|/Script/Engine.SceneComponent|GetRelativeRotation (Variables|Default|GetCapsuleComponent)) "TraceTypeQuery1" false 0 "Persistent"))
  (if _returnvalue
    (Rendering|SetVisibility (Variables|Default|GetCable) true false)
    (Class|CableComponent|SetAttachEndto _cable (.HitActor (Collision|BreakHitResult _outhit)) "None" "None")
    (Utilities|FlowControl|Delay 1.0)
    (Rendering|SetVisibility _cable false false)))

(event Input|EnhancedActionEvents|EnhancedInputActionIA_Jump
  (params (ActionValue :type Boolean) (ElapsedSeconds :type Float%20%28double-precision%29) (TriggeredSeconds :type Float%20%28double-precision%29) (InputAction :type Input%20Action%20Object%20Reference :default "/Game/CoreGame/Input/Actions/IA_Jump.IA_Jump"))
  (:Triggered
    (CallFunction|DoJump))
  (:Completed
    (CallFunction|StopJump)))

(event Input|EnhancedActionEvents|EnhancedInputActionIA_UniqueAttack2
  (params (ActionValue :type Boolean) (ElapsedSeconds :type Float%20%28double-precision%29) (TriggeredSeconds :type Float%20%28double-precision%29) (InputAction :type Input%20Action%20Object%20Reference :default "/Game/CoreGame/Input/Actions/IA_UniqueAttack2.IA_UniqueAttack2"))
  (:Triggered
    (CallFunction|Pull)))

(event Input|EnhancedActionEvents|EnhancedInputActionIA_Kick
  (params (ActionValue :type Boolean) (ElapsedSeconds :type Float%20%28double-precision%29) (TriggeredSeconds :type Float%20%28double-precision%29) (InputAction :type Input%20Action%20Object%20Reference :default "/Game/CoreGame/Input/Actions/IA_Kick.IA_Kick"))
  (:Triggered
    (CallFunction|DoKick)))

(event Input|EnhancedActionEvents|EnhancedInputActionIA_Punch
  (params (ActionValue :type Boolean) (ElapsedSeconds :type Float%20%28double-precision%29) (TriggeredSeconds :type Float%20%28double-precision%29) (InputAction :type Input%20Action%20Object%20Reference :default "/Game/CoreGame/Input/Actions/IA_Punch.IA_Punch"))
  (:Triggered
    (CallFunction|DoPunch)))

(event Input|EnhancedActionEvents|EnhancedInputActionIA_UniqueAttack1
  (params (ActionValue :type Boolean) (ElapsedSeconds :type Float%20%28double-precision%29) (TriggeredSeconds :type Float%20%28double-precision%29) (InputAction :type Input%20Action%20Object%20Reference :default "/Game/CoreGame/Input/Actions/IA_UniqueAttack1.IA_UniqueAttack1"))
  (:Triggered
    (CallFunction|Bash)))

(event Input|EnhancedActionEvents|EnhancedInputActionIA_Emote
  (params (ActionValue :type Boolean) (ElapsedSeconds :type Float%20%28double-precision%29) (TriggeredSeconds :type Float%20%28double-precision%29) (InputAction :type Input%20Action%20Object%20Reference :default "/Game/CoreGame/Input/Actions/IA_Emote.IA_Emote"))
  (:Triggered
    (CallFunction|DoEmote)))

(event Input|EnhancedActionEvents|EnhancedInputActionIA_Pause
  (params (ActionValue :type Boolean) (ElapsedSeconds :type Float%20%28double-precision%29) (TriggeredSeconds :type Float%20%28double-precision%29) (InputAction :type Input%20Action%20Object%20Reference :default "/Game/CoreGame/Input/Actions/IA_Pause.IA_Pause")))

(event Input|EnhancedActionEvents|EnhancedInputActionIA_Block
  (params (ActionValue :type Boolean) (ElapsedSeconds :type Float%20%28double-precision%29) (TriggeredSeconds :type Float%20%28double-precision%29) (InputAction :type Input%20Action%20Object%20Reference :default "/Game/CoreGame/Input/Actions/IA_Block.IA_Block"))
  (:Triggered
    (CallFunction|DoBlock))
  (:Canceled
    (CallFunction|DoBlockStop :!label _label))
  (:Completed
    (goto _label)))

(event EventBeginPlay
  (bind _mesh (Variables|Character|GetMesh))
  (Utilities|FlowControl|DelayUntilNextTick)
  (bind _returnvalue (Game|SpawnActorfromClass "/Game/Characters/Hats/BP_Horns.BP_Horns_C" (Transformation|GetSocketTransform _mesh "HeadSocket" "RTS_World") "Undefined" "MultiplyWithRoot" 0 0))
  (Transformation|AttachComponentToComponent _returnvalue _mesh "HeadSocket" "SnapToTarget" "SnapToTarget" "SnapToTarget" true))

(fn ConstructionScript
  (|CallParentFunction))