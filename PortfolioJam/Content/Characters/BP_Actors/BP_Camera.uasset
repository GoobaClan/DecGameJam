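; Camera actor that follows two player characters by staying centred between them at a fixed offset.
; Every tick it gathers all BP_Character actors, storing the first location as Player1 and any later one as Player2.
; It moves to their midpoint, via a sinusoidal ease at half alpha, shifted back along world X and up.
; Movement is immediate, with no smoothing over time or rotation change.
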(event EventTick
  (params (DeltaSeconds :type Float%20%28single-precision%29))
  (bind _outactors (Actor|GetAllActorsOfClass "/Game/Characters/BP_Character.BP_Character_C"))
  (for (_array_element _array_index) _outactors
    (if (== _array_index 0)
      (Variables|Default|SetPlayer1 (Transformation|GetActorLocation _array_element))
      (else
        (Variables|Default|SetPlayer2 (Transformation|GetActorLocation _array_element)))))
  (Transformation|SetActorLocation (+ (Math|Interpolation|Ease "SinusoidalInOut" 0.5 (Variables|Default|GetPlayer1) (Variables|Default|GetPlayer2)) "-1000.000000,0.000000,1000.000000") false false))

(fn ConstructionScript)